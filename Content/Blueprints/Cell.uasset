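; Cell is a board square in a projectile-driven tic-tac-toe style game, claimed as cross or circle when hit.
; On a Cube hit it checks each SupportController's turn and game state, matching the projectile by component name to claim an empty cell and flip the turn.
; Tick shows or hides the CrossCube and CircleCube meshes according to CurrentState.
; GetIsCross is an empty stub.
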(event `self.Cube.OnComponentHit`
  (params (HitComponent :type "PrimitiveComponent Object Reference") (OtherActor :type "Actor Object Reference") (OtherComp :type "PrimitiveComponent Object Reference") (NormalImpulse :type "Vector Structure") (Hit :type "HitResult Structure (by ref)"))
  (bind _is_cross_local (`self.Is Cross Local`))
  (bind _support_controller_local (`self.Support Controller Local`))
  (bind _returnvalue (== (`self.Current State`) 0))
  (bind _returnvalue_2 (== (`self.Game State Local`) 0))
  (bind _outactors (`GameplayStatics.GetAllActorsOfClass` "/Game/Blueprints/SupportController.SupportController_C"))
  (for _array_element _outactors
    (bind _output_get (set `self.Support Controller Local` _array_element))
    (set `self.Is Cross Local` (`/Game/Blueprints/SupportController.Is Cross` _output_get))
    (set `self.Game State Local` (`/Game/Blueprints/SupportController.Game State` _output_get))
    (if (`KismetStringLibrary.EqualEqual_StrStr` "SphereProjectile1" (`KismetStringLibrary.Conv_ObjectToString` OtherComp))
      (if _returnvalue
        (if _is_cross_local
          (if _returnvalue_2
            (set `self.Current State` 1)
            (set `/Game/Blueprints/SupportController.Is Cross` false _support_controller_local))))
      (elif (`KismetStringLibrary.EqualEqual_StrStr` (`KismetStringLibrary.Conv_ObjectToString` OtherComp) "SphereProjectile2")
        (if _returnvalue
          (if (not _is_cross_local)
            (if _returnvalue_2
              (set `self.Current State` 2)
              (set `/Game/Blueprints/SupportController.Is Cross` true _support_controller_local))))))))

(event `self.ReceiveTick`
  (params (DeltaSeconds :type "Float (single-precision)"))
  (switch `int` (`self.Current State`)
    (:`0`
      (`SceneComponent.SetHiddenInGame` (`self.CrossCube`) true false)
      (`SceneComponent.SetHiddenInGame` (`self.CircleCube`) true false))
    (:`1`
      (`SceneComponent.SetHiddenInGame` (`self.CrossCube`) false false)
      (`SceneComponent.SetHiddenInGame` (`self.CircleCube`) true false))
    (:`2`
      (`SceneComponent.SetHiddenInGame` (`self.CrossCube`) true false)
      (`SceneComponent.SetHiddenInGame` (`self.CircleCube`) false false))))

(fn `Get Is Cross`)

(fn `UserConstructionScript`)