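; Player pawn that moves and looks around via axis input and fires projectiles when pointing at a cell.
; On begin play it attaches a spawned Pointer to PointerLocation and adds an Aim widget unless a head-mounted display is enabled.
; The Point action line-traces from the camera and, on a hit, spawns Projectile1 or Projectile2 by PlayerID at ShootLocation, routed through paired spawn and "Multi" events.
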(event `Spawn Projectile 1`
  (params (NewParam :type "Transform Structure"))
  (`self.Spawn Projectile 1 Multi` NewParam))

(event `Spawn Projectile 1 Multi`
  (params (NewParam :type "Transform Structure"))
  (`|SpawnActorFromClass` "/Game/Blueprints/Projectile1.Projectile1_C" NewParam "Undefined" "OverrideRootScale" null null))

(event `InputAction|Point`
  (params (Key :type "Key Structure"))
  (bind _camera (`self.Camera`))
  (bind _shootlocation (`self.ShootLocation`))
  (bind _returnvalue (`SceneComponent.K2_GetComponentLocation` _camera))
  (bind _returnvalue_2 (`KismetMathLibrary.MakeTransform` (`SceneComponent.K2_GetComponentLocation` _shootlocation) (`SceneComponent.K2_GetComponentRotation` _shootlocation) (0.1 0.1 0.1)))
  ;[1 1 1] Поинтинг нажатия на клетку
  (:`Pressed`
    (bind (_outhit _returnvalue_3) (`KismetSystemLibrary.LineTraceSingle` _returnvalue (+ _returnvalue (* (`SceneComponent.GetForwardVector` _camera) 5000.0)) "TraceTypeQuery1"))
    (if _returnvalue_3
      ;;[1 1 1] Выбор типа напр. снаряда в зависимости от игрока
      (if (== (`self.Player ID`) 1)
        (`self.Spawn Projectile 1` _returnvalue_2)
        (else
          (`self.Spawn Projectile 2` _returnvalue_2))))))

(event `Spawn Projectile 2`
  (params (NewParam :type "Transform Structure"))
  (`self.Spawn Projectile 2 Multi` NewParam))

(event `Spawn Projectile 2 Multi`
  (params (NewParam :type "Transform Structure"))
  (`|SpawnActorFromClass` "/Game/Blueprints/Projectile2.Projectile2_C" NewParam "Undefined" "OverrideRootScale" null null))

(event `self.ReceiveBeginPlay`
  ;[1 1 1] Наложение прицела на экран и привязка указателя к игроку
  (bind _returnvalue (`|CreateWidget` "/Game/Blueprints/Aim.Aim_C"))
  (if (not (`HeadMountedDisplayFunctionLibrary.IsHeadMountedDisplayEnabled`))
    (`UserWidget.AddToPlayerScreen` _returnvalue 0))
  (bind _returnvalue_2 (`|SpawnActorFromClass` "/Game/Blueprints/Pointer.Pointer_C" (`KismetMathLibrary.MakeTransform` (0.0 0.0 0.0)) "Undefined" "OverrideRootScale" null null))
  (bind _output_get (set `self.Equipped Pointer` _returnvalue_2))
  (`self.K2_AttachToComponent` _output_get (`self.PointerLocation`) "None" "KeepRelative" "KeepRelative" "KeepRelative" true)
  (`KismetSystemLibrary.Delay` 1.0))

(event `InputAxis|ForwardMovement`
  (params (AxisValue :type "Float (single-precision)"))
  ;[1 1 1] Передвижение и поворот камеры
  ;;[1 1 1] Передвижение (клавиатура)
  (`self.AddMovementInput` (`KismetMathLibrary.GetForwardVector` (`KismetMathLibrary.MakeRotator` 0.0 0.0 (.yaw (`self.GetControlRotation`)))) AxisValue))

(event `InputAxis|SideMovement`
  (params (AxisValue :type "Float (single-precision)"))
  ;[1 1 1] Передвижение и поворот камеры
  ;;[1 1 1] Передвижение (клавиатура)
  (`self.AddMovementInput` (`KismetMathLibrary.GetRightVector` (`KismetMathLibrary.MakeRotator` 0.0 0.0 (.yaw (`self.GetControlRotation`)))) AxisValue))

(event `InputAxis|Turn`
  (params (AxisValue :type "Float (single-precision)"))
  ;[1 1 1] Передвижение и поворот камеры
  ;;[1 1 1] Поворот камеры
  (`self.AddControllerYawInput` AxisValue))

(event `InputAxis|Look Up`
  (params (AxisValue :type "Float (single-precision)"))
  ;[1 1 1] Передвижение и поворот камеры
  ;;[1 1 1] Поворот камеры
  (`self.AddControllerPitchInput` AxisValue))

(fn `UserConstructionScript`)